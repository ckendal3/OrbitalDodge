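; Background Blueprint for a map whose material continuously shifts colour and emissive glow.
; The construction script creates a dynamic material instance of BackgroundColor on the Blah component and stores it as ChangingMaterial.
; Three seconds after BeginPlay, two timelines drive the ChangingColor vector and EmissivePower scalar parameters on that instance.
; Each timeline calls its own event again on finishing, so both loop indefinitely and independently.
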(event `self.ReceiveBeginPlay`
  (`KismetSystemLibrary.Delay` 3.0)
  (`|ExecutionSequence`
    (:`then_0`
      (`self.ChangeBackgroundColor`))
    (:`then_1`
      (`self.EmissivePowerChange`))))

(event `ChangeBackgroundColor`
  (bind (_direction _colorchangingtrack) (`Timeline|ChangingColor` :!via `PlayFromStart`)
    (:`Update`
      (`MaterialInstanceDynamic.SetVectorParameterValue` (`self.ChangingMaterial`) "ChangingColor" _colorchangingtrack))
    (:`Finished`
      (`self.ChangeBackgroundColor`))))

(event `EmissivePowerChange`
  (bind (_direction _emissivepower) (`Timeline|ChangeEmissivePower` :!via `PlayFromStart`)
    (:`Update`
      (`MaterialInstanceDynamic.SetScalarParameterValue` (`self.ChangingMaterial`) "EmissivePower" _emissivepower))
    (:`Finished`
      (`self.EmissivePowerChange`))))

(fn `UserConstructionScript`
  (bind _returnvalue (`PrimitiveComponent.CreateDynamicMaterialInstance` (`self.Blah`) 0 "/Game/ObstaclesPowerups/Material/BackgroundColor.BackgroundColor"))
  (set `self.ChangingMaterial` _returnvalue))